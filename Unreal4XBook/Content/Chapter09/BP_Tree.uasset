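; BP_Tree is a tree actor that picks a random tree type for itself.
; Its construction script draws a random index from the tree type enum's entry count and stores it as RandomTreeType.
; On BeginPlay it prints the chosen type's name to the screen as formatted text.
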(event `self.ReceiveBeginPlay`
  (`KismetSystemLibrary.PrintString` (`KismetTextLibrary.Conv_TextToString` (`|FormatText` "My Type is {0}" (`KismetTextLibrary.Conv_NameToText` (`|GetEnumeratorName` (`self.RandomTreeType`)))))))

(fn `UserConstructionScript`
  (set `self.RandomTreeType` (cast `TreeType` (`KismetMathLibrary.Conv_IntToByte` (`KismetMathLibrary.RandomInteger` (enumcount `TreeType`))))))